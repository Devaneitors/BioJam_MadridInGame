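; Duck enemy character that chases through its AI Blackboard and freezes under the player's flash.
; Pawn sensing or Sphere overlap sets the hassSeenPlayer key, and leaving VisionRadio clears it.
; While the player overlaps the capsule with BCFlash on, Tick zeroes walk speed and quacks once, otherwise restoring speed and re-arming the quack.
; Tick also plays footstep sounds on a timer while moving.
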(event `self.ReceiveBeginPlay`
  (set `CharacterMovementComponent.MaxWalkSpeed` (`self.WalkSpeed`) (`self.CharacterMovement`)))

(event `self.PawnSensing.OnSeePawn`
  (params (Pawn :type "Pawn Object Reference"))
  (cast `/Game/FirstPerson/Blueprints/BP_FirstPersonCharacter` Pawn)
  (`BlackboardComponent.SetValueAsBool` (`AIBlueprintHelperLibrary.GetBlackboard` (`AIBlueprintHelperLibrary.GetAIController` self)) "hassSeenPlayer" true))

(event `self.ReceiveTick`
  (params (DeltaSeconds :type "Float (single-precision)"))
  (`|ExecutionSequence`
    (:`then_0`
      (if (`self.isInVision`)
        (bind _asbp_first_person_character (cast `/Game/FirstPerson/Blueprints/BP_FirstPersonCharacter` (`GameplayStatics.GetPlayerCharacter` 0)))
        (if (`/Game/Models/BC_FlashLight.On?` (`/Game/FirstPerson/Blueprints/BP_FirstPersonCharacter.BC_Flash` _asbp_first_person_character))
          (set `CharacterMovementComponent.MaxWalkSpeed` 0.0 (`self.CharacterMovement`))
          (`/Engine/EditorBlueprintResources/StandardMacros.DoOnce` false :!label _label
            (:`Completed`
              (`GameplayStatics.PlaySoundAtLocation` "/Game/Audio/Extra/madridingame_biojam_quack2.madridingame_biojam_quack2" (`self.K2_GetActorLocation`) (struct) 0.6 1.0 0.0 "/Game/Audio/_ATT_Profiles/ATT_PhysicsHit.ATT_PhysicsHit" null null null)))
          (else
            (set `CharacterMovementComponent.MaxWalkSpeed` (`self.WalkSpeed`) (`self.CharacterMovement`) :!label _label_2)
            (goto _label :!via `Reset`)))
        (else
          (goto _label_2))))
    (:`then_1`
      ;[1 1 1] Comment
      (bind _output_get (set `self.ActualStepInterval` (+ (`self.ActualStepInterval`) DeltaSeconds)))
      (if (and (> (`KismetMathLibrary.VSize` (`self.GetVelocity`)) 0.0) (> _output_get (* (`self.FootStepInterval`) (`KismetMathLibrary.VSize` (`KismetMathLibrary.ClampVectorSize` (`self.GetVelocity`) 0.0 1.0)))))
        (set `self.ActualStepInterval` 0.0)
        (`GameplayStatics.PlaySoundAtLocation` "/Game/Audio/Extra/madridingame_biojam_paso1.madridingame_biojam_paso1" (`self.K2_GetActorLocation`) (struct) 0.5 1.0 0.0 "/Game/Audio/_ATT_Profiles/ATT_PhysicsHit.ATT_PhysicsHit" null null null)))))

(event `self.CapsuleComponent.OnComponentBeginOverlap`
  (params (OverlappedComponent :type "PrimitiveComponent Object Reference") (OtherActor :type "Actor Object Reference") (OtherComp :type "PrimitiveComponent Object Reference") (OtherBodyIndex :type Integer) (bFromSweep :type Boolean) (SweepResult :type "HitResult Structure (by ref)"))
  (cast `/Game/FirstPerson/Blueprints/BP_FirstPersonCharacter` OtherActor)
  (set `self.isInVision` true))

(event `self.CapsuleComponent.OnComponentEndOverlap`
  (params (OverlappedComponent :type "PrimitiveComponent Object Reference") (OtherActor :type "Actor Object Reference") (OtherComp :type "PrimitiveComponent Object Reference") (OtherBodyIndex :type Integer))
  (cast `/Game/FirstPerson/Blueprints/BP_FirstPersonCharacter` OtherActor)
  (set `self.isInVision` false))

(event `self.Sphere.OnComponentBeginOverlap`
  (params (OverlappedComponent :type "PrimitiveComponent Object Reference") (OtherActor :type "Actor Object Reference") (OtherComp :type "PrimitiveComponent Object Reference") (OtherBodyIndex :type Integer) (bFromSweep :type Boolean) (SweepResult :type "HitResult Structure (by ref)"))
  (cast `/Game/FirstPerson/Blueprints/BP_FirstPersonCharacter` OtherActor)
  (`BlackboardComponent.SetValueAsBool` (`AIBlueprintHelperLibrary.GetBlackboard` (`AIBlueprintHelperLibrary.GetAIController` self)) "hassSeenPlayer" true))

(event `self.VisionRadio.OnComponentEndOverlap`
  (params (OverlappedComponent :type "PrimitiveComponent Object Reference") (OtherActor :type "Actor Object Reference") (OtherComp :type "PrimitiveComponent Object Reference") (OtherBodyIndex :type Integer))
  (cast `/Game/FirstPerson/Blueprints/BP_FirstPersonCharacter` OtherActor)
  (`BlackboardComponent.SetValueAsBool` (`AIBlueprintHelperLibrary.GetBlackboard` (`AIBlueprintHelperLibrary.GetAIController` self)) "hassSeenPlayer" false))

(fn `UserConstructionScript`)