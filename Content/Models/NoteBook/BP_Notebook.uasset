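; BP_Notebook is a selectable notebook actor that shows or hides an item info screen.
; On BeginPlay it creates a WB_ItemInfo widget and hands it a reference to itself.
; SelectItem toggles the widget on the viewport via a Selected flag, playing a paper sound each way.
; It freezes the game while the widget is open by setting global time dilation to zero, restoring it on close.
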(event `self.ReceiveBeginPlay`
  (bind _returnvalue (`|CreateWidget` "/Game/FirstPerson/Blueprints/WB_ItemInfo.WB_ItemInfo_C"))
  (bind _output_get (set `self.WidgetItemInfo` _returnvalue))
  (set `/Game/FirstPerson/Blueprints/WB_ItemInfo.noteBook` self _output_get))

(event `SelectItem`
  (bind _widgetiteminfo (`self.WidgetItemInfo`))
  (if (`self.Selected`)
    (`Widget.RemoveFromParent` _widgetiteminfo)
    (set `self.Selected` false)
    (`GameplayStatics.SetGlobalTimeDilation` 1.0)
    (`GameplayStatics.PlaySound2D` "/Game/Audio/Paper/Paper03.Paper03" 1.0 1.0 0.0 null null)
    (else
      (`UserWidget.AddToViewport` _widgetiteminfo 0)
      (set `self.Selected` true)
      (`GameplayStatics.SetGlobalTimeDilation` 0.0)
      (`GameplayStatics.PlaySound2D` "/Game/Audio/Paper/Paper04.Paper04" 1.0 1.0 0.0 null null))))

(fn `UserConstructionScript`)